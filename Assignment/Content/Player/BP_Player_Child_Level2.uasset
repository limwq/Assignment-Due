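; Level 2 first-person player child Blueprint that handles pausing, typing audio and the level's fail and victory transitions.
; BeginPlay sets game-only input and creates the scene fader and pause manager widgets; P pauses, and holding Interact plays a typing sound.
; Failed freezes the player and pitches body and view 90 degrees before fading to the fail destination, while VictoryScene fades to victory.
; Laptop and enemy line-trace logic remains but is unconnected.
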(event `Key|P`
  (params (Key :type "Key Structure"))
  (:`Pressed`
    (`/Game/FirstPerson/Blueprints/WBP_PauseManager.PauseGame` (`self.PauseManage`))))

(event `self.ReceiveTick`
  (params (DeltaSeconds :type "Float (single-precision)")))

(event `self.ReceiveBeginPlay`
  (bind _returnvalue (`GameplayStatics.GetPlayerController` 0))
  (`WidgetBlueprintLibrary.SetInputMode_GameOnly` _returnvalue)
  (`self.EnableInput` _returnvalue)
  (bind _returnvalue_2 (`|CreateWidget` "/Game/FirstPerson/Blueprints/WBP_SceneFader.WBP_SceneFader_C"))
  (bind _output_get (set `self.SceneFade` _returnvalue_2))
  (`UserWidget.AddToViewport` _output_get 100)
  (`/Game/FirstPerson/Blueprints/WBP_SceneFader.PlayFadeIn` _output_get)
  (bind _returnvalue_3 (`|CreateWidget` "/Game/FirstPerson/Blueprints/WBP_PauseManager.WBP_PauseManager_C"))
  (bind _output_get_2 (set `self.PauseManage` _returnvalue_3))
  (`UserWidget.AddToViewport` _output_get_2 100))

(event `InputAction|Interact`
  (params (Key :type "Key Structure"))
  (bind _soundcue (`self.SoundCue`))
  (:`Pressed`
    (`|ExecutionSequence`
      (:`then_1`
        (if (not (`KismetSystemLibrary.IsValid` (`self.SoundCue`)))
          (bind _returnvalue (`GameplayStatics.SpawnSound2D` "/Game/Sprite-Audio/ItemAudio/keyboard-typing-effect-free-393912.keyboard-typing-effect-free-393912" 0.3 1.0 0.0 null))
          (set `self.SoundCue` _returnvalue)))))
  (:`Released`
    (if (`KismetSystemLibrary.IsValid` (`self.SoundCue`))
      (`AudioComponent.Stop` _soundcue)
      (`ActorComponent.K2_DestroyComponent` _soundcue))))

(event `Failed`
  (bind (_returnvalue_roll _returnvalue_pitch _returnvalue_yaw) (`KismetMathLibrary.BreakRotator` (`self.K2_GetActorRotation`)))
  (bind (_returnvalue_x _returnvalue_y _returnvalue_z) (`KismetMathLibrary.BreakVector` (`self.K2_GetActorLocation`)))
  (bind _returnvalue (+ _returnvalue_pitch 90.0))
  (`self.DisableInput` (`GameplayStatics.GetPlayerController` 0))
  (`CharacterMovementComponent.SetMovementMode` (`self.CharacterMovement`) "MOVE_None" 0)
  (`self.K2_SetActorLocationAndRotation` (`KismetMathLibrary.MakeVector` _returnvalue_x _returnvalue_y (+ _returnvalue_z 5.0)) (`KismetMathLibrary.MakeRotator` _returnvalue_roll _returnvalue _returnvalue_yaw))
  (`Controller.SetControlRotation` (`GameplayStatics.GetPlayerController` 0) (`KismetMathLibrary.MakeRotator` _returnvalue_roll _returnvalue _returnvalue_yaw))
  (`KismetSystemLibrary.Delay` 1.0)
  (`/Game/FirstPerson/Blueprints/WBP_SceneFader.PlayFadeOut` (`self.SceneFade`))
  (`KismetSystemLibrary.Delay` 1.0)
  (`SceneManager.GoToFail` (`GameplayStatics.GetPlayerController` 0)))

(event `VictoryScene`
  (`KismetSystemLibrary.Delay` 1.0)
  (`/Game/FirstPerson/Blueprints/WBP_SceneFader.PlayFadeOut` (`self.SceneFade`))
  (`KismetSystemLibrary.Delay` 1.0)
  (`SceneManager.GoToVictory` (`GameplayStatics.GetPlayerController` 0)))

(fn `UserConstructionScript`
  (`parent.UserConstructionScript`))