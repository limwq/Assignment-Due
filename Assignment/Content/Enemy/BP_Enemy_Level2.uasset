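; BP_Enemy_Level2 is an enemy character that slowly chases the player.
; BeginPlay sets a very low max walk speed on the CharacterMovement component.
; Each Tick feeds the unnormalized vector toward player 0's pawn into AddMovementInput, steering directly with no pathfinding, then prints the current speed for debugging.
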(event `self.ReceiveBeginPlay`
  (set `CharacterMovementComponent.MaxWalkSpeed` 5.0 (`self.CharacterMovement`)))

(event `self.ReceiveTick`
  (params (DeltaSeconds :type "Float (single-precision)"))
  (`|ExecutionSequence`
    (:`then_0`
      (`self.AddMovementInput` (- (`self.K2_GetActorLocation` (`GameplayStatics.GetPlayerPawn` 0)) (`self.K2_GetActorLocation`))))
    (:`then_1`
      (`KismetSystemLibrary.PrintString` (`KismetStringLibrary.Conv_DoubleToString` (`KismetMathLibrary.VSize` (`self.GetVelocity`)))))))

(fn `UserConstructionScript`
  (`parent.UserConstructionScript`))